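; Spider character that wanders randomly on the navmesh and can be picked up and dropped.
; After a startup fall animation, Tick starts AIMoveTo toward random reachable points with short rests between, toggling ABP_Spider's walk flag, and draws a debug sphere.
; Pickup attaches only the mesh to the given component.
; Drop traces to the ground, moves the capsule there, reattaches the mesh at its saved offset with physics enabled, then briefly pauses wandering.
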(event EventTick
  (params (DeltaSeconds :type Float%20%28single-precision%29))
  (bind _mesh (Variables|Character|GetMesh))
  (bind _returnvalue (Components|SkeletalMesh|GetAnimInstance _mesh))
  (Utilities|FlowControl|Sequence
    (:then_0
      (Rendering|Debug|DrawDebugSphere (Transformation|GetWorldLocation (Variables|Character|GetMesh)) 1e+01 12 "(R=1.000000,G=0.000000,B=0.734106,A=1.000000)" 0.0))
    (:then_1
      (if (Math|Boolean|ANDBoolean (not (Variables|Default|GetIsWalking)) (not (Variables|Default|GetIsPickedUp)) (not (Variables|Default|GetWaitABit)))
        (CallFunction|SetNextRandomPosition)
        (AI|AIMoveTo self (Variables|Default|GetNextDestination) 0 5.0 (Variables|Default|GetIsPickedUp)
          (:then
            (Variables|Default|SetIsWalking true)
            (bind _asabp_spider (Utilities|Casting|CastToABP_Spider _returnvalue))
            (Variables|/Game/MyContent/Spider/ABP_Spider.ABP_Spider_C|SetCanWalk _asabp_spider true))
          (:OnSuccess
            (bind _asabp_spider_2 (Utilities|Casting|CastToABP_Spider _returnvalue :!label _label))
            (Variables|/Game/MyContent/Spider/ABP_Spider.ABP_Spider_C|SetCanWalk _asabp_spider_2 false)
            (Variables|Default|SetWaitABit true)
            (Utilities|FlowControl|Delay (Math|Random|RandomFloatinRange 2.0 3.0))
            (Variables|Default|SetWaitABit false)
            (Variables|Default|SetIsWalking false)
            (CallFunction|SetNextRandomPosition))
          (:OnFail
            (goto _label)))))))

(event EventPickup
  (params (AttachTo :type Scene%20Component%20Object%20Reference))
  (bind _mesh (Variables|Character|GetMesh))
  (Variables|Default|SetOffsetMeshHeight (- (Transformation|GetWorldLocation (Variables|Character|GetMesh)) (Transformation|GetWorldLocation (Variables|Collision|GetCapsuleComponent))))
  (Variables|Default|SetIsWalking false)
  (Variables|Default|SetIsPickedUp true)
  (Physics|SetSimulatePhysics _mesh false)
  (Transformation|AttachComponentToComponent _mesh AttachTo "None" "KeepWorld" "KeepWorld" "KeepWorld" false))

(event EventDrop
  (CallFunction|ReleaseSpider)
  (Variables|Default|SetWaitABit true)
  (Utilities|FlowControl|Delay 2.0)
  (Variables|Default|SetWaitABit false)
  (Variables|Default|SetIsWalking false)
  (Variables|Default|SetIsPickedUp false))

(event EventBeginPlay
  (Variables|Default|SetWaitABit true)
  (bind _asabp_spider (Utilities|Casting|CastToABP_Spider (Components|SkeletalMesh|GetAnimInstance (Variables|Character|GetMesh))))
  (Variables|/Game/MyContent/Spider/ABP_Spider.ABP_Spider_C|SetStartFall _asabp_spider true)
  (Utilities|FlowControl|Delay 1.0)
  (Variables|/Game/MyContent/Spider/ABP_Spider.ABP_Spider_C|SetStartFall _asabp_spider false)
  (Utilities|FlowControl|Delay 2.0)
  (Variables|Default|SetWaitABit false)
  (bind _output_get (Variables|Default|SetWalkingSpeed (Math|Random|RandomFloatinRange 2e+01 3e+01)))
  (Variables|/Script/Engine.CharacterMovementComponent|SetMaxWalkSpeed (Variables|Character|GetCharacterMovement) _output_get))

(fn ConstructionScript)

(fn ReleaseSpider
  (bind _mesh (Variables|Character|GetMesh))
  (bind _capsulecomponent (Variables|Collision|GetCapsuleComponent))
  (bind _mesh_2 (Variables|Character|GetMesh))
  (Physics|SetSimulatePhysics _mesh true)
  (Transformation|DetachFromComponent _mesh "KeepWorld" "KeepWorld" "KeepWorld" true)
  (bind _groundposition (CallFunction|GetGroundBelow _mesh_2 _capsulecomponent))
  (Transformation|SetWorldLocationAndRotation (Variables|Collision|GetCapsuleComponent) _groundposition "0, 0, 0" false false)
  (Physics|SetEnableGravity _mesh true)
  (Class|SkeletalMeshComponent|SetEnableGravityonAllBodiesBelow _mesh true "None" true)
  (Transformation|AttachComponentToComponent _mesh _capsulecomponent "None" "KeepWorld" "KeepWorld" "KeepWorld" true)
  (Transformation|SetWorldLocationAndRotation _mesh_2 (+ _groundposition (Variables|Default|GetOffsetMeshHeight)) "0.0,-90.000000,0.0" false false)
  (Physics|SetSimulatePhysics _mesh true)
  ;[1 1 1] compute new ia target
  (CallFunction|SetNextRandomPosition))

(fn GetGroundBelow
  (params (Mesh :type Mesh%20Component%20Object%20Reference) (ParentComponent :type Primitive%20Component%20Object%20Reference))
  (bind _returnvalue (Transformation|GetWorldLocation Mesh))
  (bind _outhit (Collision|LineTraceByChannel _returnvalue (+ _returnvalue (* (Math|Vector|NegateVector (Transformation|GetActorUpVector)) 1.5e+03)) "TraceTypeQuery1" false (Collision|GetOverlappingActors ParentComponent 0 :!class /Script/Engine.PrimitiveComponent) "None"))
  (return (.Location (Collision|BreakHitResult _outhit))))

(fn SetNextRandomPosition
  (Variables|Default|SetNextDestination (.RandomLocation (Class|NavigationSystem|GetRandomPointinNavigableRadius (Transformation|GetActorLocation) (Variables|Default|GetWalkRadius))))
  (return))